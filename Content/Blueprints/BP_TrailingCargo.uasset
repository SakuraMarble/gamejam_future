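; BP_TrailingCargo is a cargo actor that trails behind a follow target for a Snake-game style chain effect.
; Each Tick it interpolates toward the target's position, offset back along world X by FollowDistance, without sweeping; the IsValid check on the target is left unconnected.
; The construction script creates a dynamic instance of the BoxA material on StaticMesh1 and applies the Color variable to it.
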(event `self.ReceiveTick`
  (params (DeltaSeconds :type "Float (single-precision)"))
  (bind (_returnvalue_x _returnvalue_y _returnvalue_z) (`KismetMathLibrary.BreakVector` (`self.K2_GetActorLocation` (`self.FollowTarget`))))
  ;[1 1 1] 实现“贪吃蛇”效果，货物跟随
  (`self.K2_SetActorLocation` (`KismetMathLibrary.VInterpTo` (`self.K2_GetActorLocation`) (`KismetMathLibrary.MakeVector` (- _returnvalue_x (`self.FollowDistance`)) _returnvalue_y _returnvalue_z) DeltaSeconds (`self.InterpSpeed`))))

(fn `UserConstructionScript`
  (bind _returnvalue (`PrimitiveComponent.CreateDynamicMaterialInstance` (`self.StaticMesh1`) 0 "/Game/Fab/Cardboard_Package_Box/BoxA.BoxA" "None"))
  (`MaterialInstanceDynamic.SetVectorParameterValue` _returnvalue "Color" (`self.Color`)))
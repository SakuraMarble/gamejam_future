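; BP_FinalPoint is the end gate that finishes the game when the player ship enters it.
; A Box overlap casts to BP_PlayerShip, waits briefly, then calls the ship's GameEndFailOrSucceed, passing the ship's own Succeessful value.
; The construction script creates dynamic instances of M_Basic_Wall on the static mesh's first two material slots and tints both with GateColor.
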(event `self.ReceiveBeginPlay`
  (add `PrimitiveComponent.OnComponentBeginOverlap` (`self.Box`) (delegate `Collison`)))

(event `Collison`
  (params (OverlappedComponent :type "PrimitiveComponent Object Reference") (OtherActor :type "Actor Object Reference") (OtherComp :type "PrimitiveComponent Object Reference") (OtherBodyIndex :type Integer) (bFromSweep :type Boolean) (SweepResult :type "HitResult Structure (by ref)"))
  (bind _asbp_player_ship (cast `/Game/Blueprints/BP_PlayerShip` OtherActor))
  (`KismetSystemLibrary.Delay` 0.4)
  (`/Game/Blueprints/BP_PlayerShip.GameEndFailOrSucceed` _asbp_player_ship (`/Game/Blueprints/BP_PlayerShip.Succeessful` _asbp_player_ship)))

(fn `UserConstructionScript`
  (bind _gatecolor (`self.GateColor`))
  (bind _returnvalue (`PrimitiveComponent.CreateDynamicMaterialInstance` (`self.StaticMesh`) 0 "/Game/StarterContent/Materials/M_Basic_Wall.M_Basic_Wall" "None"))
  (`MaterialInstanceDynamic.SetVectorParameterValue` _returnvalue "Color" _gatecolor)
  (bind _returnvalue_2 (`PrimitiveComponent.CreateDynamicMaterialInstance` (`self.StaticMesh`) 1 "/Game/StarterContent/Materials/M_Basic_Wall.M_Basic_Wall" "None"))
  (`MaterialInstanceDynamic.SetVectorParameterValue` _returnvalue_2 "Color" _gatecolor))
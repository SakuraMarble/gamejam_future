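; Floor tile for an endless ship runner that builds the track ahead as the player advances.
; On BeginPlay it spawns and attaches one random gate, pickup, meteor or sprint trigger in a random lane, randomly coloring gates and pickups.
; When BP_PlayerShip overlaps its trigger, it spawns BP_FloorTile, or BP_FinalPoint once GameDistance reaches FinalDistance, at AttachPoint.
; It destroys itself after a short delay, taking attached actors with it.
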(event `self.ReceiveBeginPlay`
  (bind _defaultsceneroot (`self.DefaultSceneRoot`))
  (bind _returnvalue (select `int` (`KismetMathLibrary.RandomIntegerInRange` 0 2) :`0` (struct :`R` 1.0 :`A` 1.0) :`1` (struct :`R` 0.951198 :`G` 1.0 :`B` 0.069846 :`A` 1.0) :`2` (struct :`R` 0.02055 :`G` 0.090904 :`B` 1.0 :`A` 1.0) :!type "LinearColor Structure"))
  (bind _returnvalue_2 (`SceneComponent.K2_GetComponentToWorld` (`|GetArrayItem` (`|MakeArray` (`self.SpawnPoint_Left`) (`self.SpawnPoint_Center`) (`self.SpawnPoint_Right`)) (`KismetMathLibrary.RandomIntegerInRange` 0 2))))
  ;[1 1 1] 无限生成地块逻辑
  (add `PrimitiveComponent.OnComponentBeginOverlap` (`self.TriggerBox`) (delegate `Collison`))
  ;[1 1 1] 随机轨道生成陨石或宝箱逻辑
  (switch `int` (`KismetMathLibrary.RandomIntegerInRange` 0 3)
    (:`0`
      (bind _returnvalue_3 (`|SpawnActorFromClass` "/Game/Blueprints/BP_Gate.BP_Gate_C" _returnvalue_2 "Undefined" "MultiplyWithRoot" null _returnvalue null))
      (`self.K2_AttachToComponent` _returnvalue_3 _defaultsceneroot "None" "KeepWorld" "KeepWorld" "KeepWorld" true))
    (:`1`
      (bind _returnvalue_4 (`|SpawnActorFromClass` "/Game/Blueprints/BP_Pickup.BP_Pickup_C" _returnvalue_2 "Undefined" "MultiplyWithRoot" null _returnvalue null))
      (`self.K2_AttachToComponent` _returnvalue_4 _defaultsceneroot "None" "KeepWorld" "KeepWorld" "KeepWorld" true))
    (:`2`
      (bind _returnvalue_5 (`|SpawnActorFromClass` "/Game/Blueprints/BP_Meteor.BP_Meteor_C" _returnvalue_2 "Undefined" "MultiplyWithRoot" null null))
      (`self.K2_AttachToComponent` _returnvalue_5 _defaultsceneroot "None" "KeepWorld" "KeepWorld" "KeepWorld" true))
    (:`3`
      (bind _returnvalue_6 (`|SpawnActorFromClass` "/Game/Blueprints/BP_SprintTrigger.BP_SprintTrigger_C" _returnvalue_2 "Undefined" "MultiplyWithRoot" null null))
      (`self.K2_AttachToComponent` _returnvalue_6 _defaultsceneroot "None" "KeepWorld" "KeepWorld" "KeepWorld" true))))

(event `Collison`
  (params (OverlappedComponent :type "PrimitiveComponent Object Reference") (OtherActor :type "Actor Object Reference") (OtherComp :type "PrimitiveComponent Object Reference") (OtherBodyIndex :type Integer) (bFromSweep :type Boolean) (SweepResult :type "HitResult Structure (by ref)"))
  (bind _returnvalue (`SceneComponent.K2_GetComponentToWorld` (`self.AttachPoint`)))
  ;[1 1 1] 无限生成地块逻辑
  (bind _asbp_player_ship (cast `/Game/Blueprints/BP_PlayerShip` OtherActor))
  (if (< (`/Game/Blueprints/BP_PlayerShip.GameDistance` _asbp_player_ship) (`self.FinalDistance`))
    (`|SpawnActorFromClass` "/Game/Blueprints/BP_FloorTile.BP_FloorTile_C" _returnvalue "Undefined" "MultiplyWithRoot" null null)
    (`KismetSystemLibrary.Delay` 2.0)
    (`self.K2_DestroyActor`)
    (else
      (`|SpawnActorFromClass` "/Game/Blueprints/BP_FinalPoint.BP_FinalPoint_C" _returnvalue "Undefined" "MultiplyWithRoot" null (struct) null)
      (`KismetSystemLibrary.Delay` 2.0)
      (`self.K2_DestroyActor`))))

(event `self.ReceiveDestroyed`
  ;[1 1 1] 销毁逻辑，确保清除垃圾
  (for _array_element (`self.GetAttachedActors` true)
    (`self.K2_DestroyActor` _array_element)))

(fn `UserConstructionScript`)
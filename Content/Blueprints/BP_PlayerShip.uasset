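; Player ship for a three-lane runner that dodges meteors, collects colored cargo and tracks score and distance.
; Tick accelerates it forward, interpolating lane position, roll and wind pitch; A/D switch lanes, W/S drive height timelines.
; Overlaps cost health, trigger FOV-widening sprints, or add cargo to a follow chain mirrored by a last-in-first-out color stack.
; Zero health pauses the game and shows the game-over widget.
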(event `self.ReceiveTick`
  (params (DeltaSeconds :type "Float (single-precision)"))
  (bind (_returnvalue_roll _returnvalue_pitch _returnvalue_yaw) (`KismetMathLibrary.BreakRotator` (`self.K2_GetActorRotation`)))
  (bind _returnvalue (`self.K2_GetActorLocation`))
  (bind (_returnvalue_x _returnvalue_y) (`KismetMathLibrary.BreakVector` (`self.K2_GetActorLocation`)))
  (bind _returnvalue_x_2 (`KismetMathLibrary.BreakVector` (`self.K2_GetActorLocation`)))
  (bind _maxtiltangle (`self.MaxTiltAngle`))
  ;[1 1 1] WASD操作逻辑
  (set `self.GameDistance` (+ _returnvalue_x_2 15000.0))
  ;[1 1 1] 自动前进与航道切换逻辑
  (set `self.CurX` (+ (* (`self.ForwardSpeed`) DeltaSeconds) (.x _returnvalue)))
  (set `self.TargetLocation` (`KismetMathLibrary.MakeVector` (`self.CurX`) (* (`self.CurrentLane`) (`self.LaneWidth`)) (`self.CurrentHeightOffset`)))
  (`self.K2_SetActorLocation` (`KismetMathLibrary.VInterpTo` _returnvalue (`self.TargetLocation`) (`GameplayStatics.GetWorldDeltaSeconds`) 7.0))
  ;[1 1 1] 加速和音调变化逻辑
  (set `self.ForwardSpeed` (`KismetMathLibrary.FClamp` (+ (`self.ForwardSpeed`) (`self.SpeedUpRate`)) (`self.MinForwardSpeed`) (`self.MaxForwardSpeed`)))
  (`AudioComponent.SetPitchMultiplier` (`self.Wind`) (`KismetMathLibrary.MapRangeClamped` (`self.ForwardSpeed`) (`self.MinForwardSpeed`) (`self.MaxForwardSpeed`) 0.1 8.0))
  ;[1 1 1] 左右ROLL
  (`self.K2_SetActorRotation` (`KismetMathLibrary.MakeRotator` (`KismetMathLibrary.FInterpTo` _returnvalue_roll (`KismetMathLibrary.MapRangeClamped` (- (.y (`self.TargetLocation`)) _returnvalue_y) -90.0 90.0 (* _maxtiltangle -1.0) _maxtiltangle) (`GameplayStatics.GetWorldDeltaSeconds`) (`self.TiltInterpSpeed`)) _returnvalue_pitch _returnvalue_yaw)))

(event `Key|D`
  (params (Key :type "Key Structure"))
  ;[1 1 1] WASD操作逻辑
  (:`Pressed`
    (set `self.CurrentLane` (`KismetMathLibrary.Clamp` (+ (`self.CurrentLane`) 1) -1 1))))

(event `Key|A`
  (params (Key :type "Key Structure"))
  ;[1 1 1] WASD操作逻辑
  (:`Pressed`
    (set `self.CurrentLane` (`KismetMathLibrary.Clamp` (- (`self.CurrentLane`) 1) -1 1))))

(event `Key|W`
  (params (Key :type "Key Structure"))
  (bind (_returnvalue_x _returnvalue_y _returnvalue_z) (`KismetMathLibrary.BreakVector` (`self.K2_GetActorLocation`)))
  ;[1 1 1] WASD操作逻辑
  (:`Pressed`
    (if (< _returnvalue_z 10.0)
      (bind (_direction _jumpoffset) (`Timeline|Timeline_Jump` :!via `PlayFromStart`)
        (:`Update`
          (set `self.CurrentHeightOffset` _jumpoffset))))))

(event `Key|S`
  (params (Key :type "Key Structure"))
  ;[1 1 1] WASD操作逻辑
  (:`Pressed`
    (bind (_direction _downoffset) (`Timeline|Timeline_Down` :!via `PlayFromStart`)
      (:`Update`
        (set `self.CurrentHeightOffset` _downoffset)))))

(event `self.ReceiveBeginPlay`
  (bind _returnvalue (`GameplayStatics.GetPlayerController` 0))
  ;[1 1 1] 生命值和死亡逻辑
  (set `PlayerController.bShowMouseCursor` false _returnvalue)
  (`WidgetBlueprintLibrary.SetInputMode_GameOnly` _returnvalue)
  (`GameplayStatics.SetGamePaused` false)
  (add `PrimitiveComponent.OnComponentBeginOverlap` (`self.StaticMesh`) (delegate `Collision_Meteor`))
  ;[1 1 1] 捡起货物逻辑
  (add `PrimitiveComponent.OnComponentBeginOverlap` (`self.StaticMesh`) (delegate `Collision_Pickup`))
  ;[1 1 1] 添加HUD
  (bind _returnvalue_2 (`|CreateWidget` "/Game/Blueprints/WBP_HUD.WBP_HUD_C" (`GameplayStatics.GetPlayerController` 0)))
  (`UserWidget.AddToViewport` _returnvalue_2 0)
  ;[1 1 1] 初始化last cargo actor
  (set `self.LastCargoActor` self)
  ;[1 1 1] 冲刺逻辑
  (add `PrimitiveComponent.OnComponentBeginOverlap` (`self.StaticMesh`) (delegate `StartSprint`)))

(event `Collision_Meteor`
  (params (OverlappedComponent :type "PrimitiveComponent Object Reference") (OtherActor :type "Actor Object Reference") (OtherComp :type "PrimitiveComponent Object Reference") (OtherBodyIndex :type Integer) (bFromSweep :type Boolean) (SweepResult :type "HitResult Structure (by ref)"))
  ;[1 1 1] 生命值和死亡逻辑
  (bind _asbp_meteor (cast `/Game/Blueprints/BP_Meteor` OtherActor))
  (`GameplayStatics.PlaySoundAtLocation` "/Game/Audio/Crash.Crash" (`self.K2_GetActorLocation` _asbp_meteor) (struct) 1.0 1.0 0.3 null null null null)
  (`GameplayStatics.SpawnEmitterAtLocation` "/Game/StarterContent/Particles/P_Explosion.P_Explosion" (`self.K2_GetActorLocation` OtherActor))
  (`self.K2_DestroyActor` _asbp_meteor)
  (set `self.Health` (- (`self.Health`) 1))
  (if (<= (`self.Health`) 0)
    (`KismetSystemLibrary.Delay` 0.4)
    (`self.GameEndFailOrSucceed` (`self.Failed`))))

(event `Collision_Pickup`
  (params (OverlappedComponent :type "PrimitiveComponent Object Reference") (OtherActor :type "Actor Object Reference") (OtherComp :type "PrimitiveComponent Object Reference") (OtherBodyIndex :type Integer) (bFromSweep :type Boolean) (SweepResult :type "HitResult Structure (by ref)"))
  ;[1 1 1] 捡起货物逻辑
  (bind _asbp_pickup (cast `/Game/Blueprints/BP_Pickup` OtherActor))
  (if (< (`KismetArrayLibrary.Array_Length` (`self.CarryingColorStack`)) (`self.MaxCargoNumber`))
    (`self.AddCargoToTrain` (`/Game/Blueprints/BP_Pickup.PickupColor` _asbp_pickup))
    (`self.K2_DestroyActor` _asbp_pickup)
    (else
      (`KismetSystemLibrary.PrintString` "最多只能载3个货物"))))

(event `StartSprint`
  (params (OverlappedComponent :type "PrimitiveComponent Object Reference") (OtherActor :type "Actor Object Reference") (OtherComp :type "PrimitiveComponent Object Reference") (OtherBodyIndex :type Integer) (bFromSweep :type Boolean) (SweepResult :type "HitResult Structure (by ref)"))
  (bind _skeletalmesh (`self.SkeletalMesh`))
  ;[1 1 1] 冲刺逻辑
  (bind _asbp_sprint_trigger (cast `/Game/Blueprints/BP_SprintTrigger` OtherActor))
  (set `self.SpeedUpRate` 0.0)
  (`SkeletalMeshComponent.PlayAnimation` _skeletalmesh "/Game/Tripo/Car/01/Run.Run" false)
  (set `self.ForwardSpeed` (+ (`self.ForwardSpeed`) (`self.SprintSpeedValue`)))
  (`self.K2_DestroyActor` _asbp_sprint_trigger)
  (bind (_direction `_新建轨道_0`) (`Timeline|平滑视场增大` :!label _label)
    (:`Update`
      (set `CameraComponent.FieldOfView` (`KismetMathLibrary.Lerp` 90.0 120.0 `_新建轨道_0`) (`self.Camera`))
      (`KismetSystemLibrary.RetriggerableDelay` 1.0)
      (`SkeletalMeshComponent.SetAnimationMode` _skeletalmesh "AnimationBlueprint" true)
      (goto _label :!via `Reverse`))
    (:`Finished`
      (switch `ETimelineDirection` _direction
        (:`Backward`
          (set `self.SpeedUpRate` (`self.SpeedUpRateConst`)))))))

(fn `AddCargoToTrain`
  (params (NewColor :type "LinearColor Structure"))
  ;[1 1 1] 添加货物到末尾：生成、颜色数组、actor数组
  (bind _returnvalue (`|SpawnActorFromClass` "/Game/Blueprints/BP_TrailingCargo.BP_TrailingCargo_C" (`self.GetTransform` (`self.LastCargoActor`)) "Undefined" "MultiplyWithRoot" null NewColor null))
  (set `/Game/Blueprints/BP_TrailingCargo.FollowTarget` (`self.LastCargoActor`) _returnvalue)
  (set `self.LastCargoActor` _returnvalue)
  (`KismetArrayLibrary.Array_Add` (`self.CargoActors`) _returnvalue)
  (`KismetArrayLibrary.Array_Add` (`self.CarryingColorStack`) NewColor))

(fn `AddScore`
  (set `self.Score` (+ (`self.Score`) (`self.SingleAddScore`))))

(fn `GameEndFailOrSucceed`
  (params (Condition :type Boolean))
  (bind _returnvalue (`GameplayStatics.GetPlayerController` 0))
  (bind _returnvalue_2 (`GameplayStatics.GetPlayerController` 0))
  (bind _gamedistance (`self.GameDistance`))
  (bind _score (`self.Score`))
  (`GameplayStatics.PlaySound2D` "/Game/Audio/GameOver.GameOver" 1.0 1.0 0.0 null null)
  (`self.OnPlayerDied`)
  (`GameplayStatics.SetGamePaused` true)
  (if Condition
    (bind _returnvalue_3 (`|CreateWidget` "/Game/Blueprints/WBP_GameOver.WBP_GameOver_C" null _score _gamedistance))
    (`UserWidget.AddToViewport` _returnvalue_3 0)
    (set `PlayerController.bShowMouseCursor` true _returnvalue)
    (`WidgetBlueprintLibrary.SetInputMode_UIOnlyEx` _returnvalue _returnvalue_3)
    (else
      (bind _returnvalue_4 (`|CreateWidget` "/Game/Blueprints/WBP_GameOver.WBP_GameOver_C" null _score _gamedistance))
      (`UserWidget.AddToViewport` _returnvalue_4 0)
      (set `PlayerController.bShowMouseCursor` true _returnvalue_2)
      (`WidgetBlueprintLibrary.SetInputMode_UIOnlyEx` _returnvalue_2 _returnvalue_4))))

(fn `PeekLastColor`
  (returns (LastColor :type "LinearColor Structure"))
  (bind _carryingcolorstack (`self.CarryingColorStack`))
  ;[1 1 1] 只是查看最后一个颜色，不移除
  (if (> (`KismetArrayLibrary.Array_Length` (`self.CarryingColorStack`)) 0)
    (return (`|GetArrayItem` _carryingcolorstack (`KismetArrayLibrary.Array_LastIndex` _carryingcolorstack)))))

(fn `PopColor`
  (bind _carryingcolorstack (`self.CarryingColorStack`))
  (bind _cargoactors (`self.CargoActors`))
  (bind _cargoactors_2 (`self.CargoActors`))
  (bind _returnvalue (`KismetArrayLibrary.Array_LastIndex` _cargoactors))
  ;[1 1 1] 移除最后一个货物。三个部分：颜色数组、actor数组、销毁，更新last货物。如果货物已经空了，last货物就设置为self；否则设置为新的末尾actor
  (if (> (`KismetArrayLibrary.Array_Length` (`self.CarryingColorStack`)) 0)
    (`KismetArrayLibrary.Array_Remove` _carryingcolorstack (`KismetArrayLibrary.Array_LastIndex` _carryingcolorstack))
    (`self.K2_DestroyActor` (`|GetArrayItem` _cargoactors _returnvalue))
    (`KismetArrayLibrary.Array_Remove` _cargoactors _returnvalue)
    (if (> (`KismetArrayLibrary.Array_Length` (`self.CargoActors`)) 0)
      (set `self.LastCargoActor` (`|GetArrayItem` _cargoactors_2 (`KismetArrayLibrary.Array_LastIndex` _cargoactors_2)))
      (else
        (set `self.LastCargoActor` self)))))

(fn `SubScore`
  (set `self.Score` (- (`self.Score`) (`self.SingleSubScore`))))

(fn `UserConstructionScript`)
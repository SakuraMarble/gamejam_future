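; Stylized Rendering System fog actor that applies height-based fog as a post-process effect, optionally limited to primary and secondary feathered box bounds.
; On construction, Refresh updates the bounds visuals and creates dynamic fog materials, with an optional translucency pass.
; It feeds them actor height, color, density, custom depth/stencil mask and bounds parameters.
; Outside packaged builds, it adds a warning material when effects quality is too low.
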(event `self.ReceiveBeginPlay`)

(fn `Check And Deploy Warnings`
  ;[1 0.729 0] No On-Screen Warnings in Packaged Projects
  (if (`KismetSystemLibrary.IsPackagedForDistribution`)
    _
    (elif (not (`self.Disable Warnings`))
      ;[1 1 1] Project Setting Warning (Custom Depth Stencil Pass)
      (bind _returnvalue (`KismetSystemLibrary.GetConsoleVariableIntValue` "sg.EffectsQuality"))
      (if (< _returnvalue 3)
        (bind _returnvalue_2 (`KismetMaterialLibrary.CreateDynamicMaterialInstance` "/Game/StylizedRenderingSystem/Materials/Private/Misc/MI_SRS_InsufficientQuality_Fog_Warning.MI_SRS_InsufficientQuality_Fog_Warning" "Main"))
        (`KismetArrayLibrary.Array_Set` (`.Array` (break `WeightedBlendables` (`.WeightedBlendables` (break `PostProcessSettings` (`PostProcessComponent.Settings` (`self.PostProcess`)))))) 0 (make `WeightedBlendable` 1.0 _returnvalue_2) true)))))

(fn `Refresh`
  (locals (`Current Fog Mat` :type "MaterialInstanceDynamic Object Reference"))
  (bind (_returnvalue_x _returnvalue_y _returnvalue_z) (`KismetMathLibrary.BreakVector` (`self.K2_GetActorLocation`)))
  (bind _postprocess (`self.PostProcess`))
  (bind _secondary_bounds_size (`self.Secondary Bounds Size`))
  (bind _secondary_bounds (`self.Secondary Bounds`))
  (bind _secondary_bounds_outer_feather (`self.Secondary Bounds Outer Feather`))
  (bind _secondary_bounds_feathering (`self.Secondary bounds Feathering`))
  (bind _primary_bounds_feather (`self.Primary Bounds Feather`))
  (bind _primary_bounds (`self.Primary Bounds`))
  (bind _current_fog_mat (`local.Current Fog Mat`))
  (`self.Check And Deploy Warnings`)
  (if (`self.Enable Fog`)
    ;[1 1 1] Limited to Bounds
    (if (`self.Use Primary Bounds`)
      (`SceneComponent.SetVisibility` _primary_bounds true false)
      (set `PostProcessComponent.bUnbound` (not (`self.Use Primary Bounds`)) _postprocess)
      (`BoxComponent.SetBoxExtent` _primary_bounds (`self.Primary Bounds Size`) true)
      (else
        (`SceneComponent.SetVisibility` _primary_bounds false false)
        (set `PostProcessComponent.bUnbound` true _postprocess)))
    ;[1 1 1] Primary Bounds Feather
    (if (and (!= (`self.Primary Bounds Feathering`) 0.0) (`self.Use Primary Bounds`))
      (`SceneComponent.SetVisibility` _primary_bounds_feather true false)
      (`BoxComponent.SetBoxExtent` _primary_bounds_feather (`KismetMathLibrary.Vector_ComponentMax` (- (`self.Primary Bounds Size`) (`self.Primary Bounds Feathering`))) true)
      (else
        (`SceneComponent.SetVisibility` _primary_bounds_feather false false)))
    ;[1 1 1] Secondary Bounds
    (if (`self.Use Secondary Bounds`)
      (`SceneComponent.SetVisibility` _secondary_bounds true false)
      (`BoxComponent.SetBoxExtent` _secondary_bounds (`self.Secondary Bounds Size`) true)
      (else
        (`SceneComponent.SetVisibility` _secondary_bounds false false)))
    ;[1 1 1] Secondary Bounds Feathering
    (if (and (!= (`self.Secondary bounds Feathering`) 0.0) (`self.Use Secondary Bounds`))
      (`SceneComponent.SetVisibility` _secondary_bounds_outer_feather true false)
      (`SceneComponent.SetVisibility` (`self.Secondary Bounds Inner Feather`) true false)
      (`BoxComponent.SetBoxExtent` (`self.Secondary Bounds Inner Feather`) (`KismetMathLibrary.Vector_ComponentMax` (- _secondary_bounds_size _secondary_bounds_feathering)) true)
      (`BoxComponent.SetBoxExtent` (`self.Secondary Bounds Outer Feather`) (+ _secondary_bounds_size _secondary_bounds_feathering) true)
      (else
        (`SceneComponent.SetVisibility` _secondary_bounds_outer_feather false false)
        (`SceneComponent.SetVisibility` (`self.Secondary Bounds Inner Feather`) false false)))
    ;[1 1 1] Create Dynamic Material Instance for Fog
    (bind _returnvalue (`KismetMaterialLibrary.CreateDynamicMaterialInstance` (`self.Fog Material`) "Main"))
    (`KismetArrayLibrary.Array_Add` (`self.Fog_Materials`) _returnvalue)
    (if (`self.Render Additional Fog Pass for Translucency`)
      (bind _returnvalue_2 (`KismetMaterialLibrary.CreateDynamicMaterialInstance` (`self.Fog Material Translucent Pass`) "Main"))
      (`KismetArrayLibrary.Array_Add` (`self.Fog_Materials`) _returnvalue_2))
    (for _array_element (`self.Fog_Materials`)
      (set `local.Current Fog Mat` _array_element)
      (`KismetArrayLibrary.Array_Add` (`.Array` (break `WeightedBlendables` (`.WeightedBlendables` (break `PostProcessSettings` (`PostProcessComponent.Settings` (`self.PostProcess`)))))) (make `WeightedBlendable` 1.0 _array_element))
      (`|ExecutionSequence`
        (:`then_0`
          (`MaterialInstanceDynamic.SetScalarParameterValue` (`local.Current Fog Mat`) "Fog Height" _returnvalue_z)
          (`MaterialInstanceDynamic.SetVectorParameterValue` (`local.Current Fog Mat`) "Fog Color" (`self.Fog Color`))
          (`MaterialInstanceDynamic.SetScalarParameterValue` (`local.Current Fog Mat`) "Fog Half Density Height" (`self.Fog Half Density Height`))
          (`MaterialInstanceDynamic.SetScalarParameterValue` (`local.Current Fog Mat`) "Camera Distance Scale" (`self.Camera Distance Scale`))
          (`MaterialInstanceDynamic.SetScalarParameterValue` (`local.Current Fog Mat`) "Use Corrected Outline Depth" (`KismetMathLibrary.Conv_BoolToDouble` (`self.Use Corrected Outline Depth`))))
        (:`then_1`
          ;[1 1 1] Custom Depth and Stencil Mask
          (`MaterialInstanceDynamic.SetScalarParameterValue` (`local.Current Fog Mat`) "Only on Custom Depth" (`KismetMathLibrary.Conv_BoolToDouble` (`self.Only on Custom Depth`)))
          (`MaterialInstanceDynamic.SetScalarParameterValue` _current_fog_mat "Stencil Mask Min" (`KismetMathLibrary.Conv_IntToDouble` (`self.Stencil Mask Min`)))
          (`MaterialInstanceDynamic.SetScalarParameterValue` _current_fog_mat "Stencil Mask Max" (`KismetMathLibrary.Conv_IntToDouble` (`self.Stencil Mask Max`))))
        (:`then_2`
          ;[1 1 1] Bounds
          (`/Game/StylizedRenderingSystem/Blueprints/Misc/BP_StylizedRenderingSystem_FunctionLibrary.SetBoundsParameters` (`local.Current Fog Mat`) self (`self.Use Primary Bounds`) (`self.Primary Bounds Size`) (`self.Primary Bounds Feathering`) (`self.Bounds Behaviour`) (`self.Use Secondary Bounds`) (`self.Secondary Bounds Size`) (`self.Secondary bounds Feathering`)))))))

(fn `UserConstructionScript`
  (`self.Refresh`))
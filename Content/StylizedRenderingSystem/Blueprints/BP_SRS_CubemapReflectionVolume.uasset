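; Stylized Rendering System volume that adds cubemap reflections through a post-process material.
; Refresh, run on construction, sizes primary and secondary feathered bounds and feeds a dynamic material the cubemap, stencil mask, bounds, reflection strength and blur settings.
; Optionally on BeginPlay, it overrides the rendering system actors' screen percentage, then captures the scene into a render target with a temporary cube capture, refreshing throughout a delay timeline before destroying it.
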(event `self.ReceiveBeginPlay`
  (bind _returnvalue (`KismetSystemLibrary.GetObjectName` self))
  (bind _returnvalue_2 (`KismetSystemLibrary.GetObjectName` self))
  (if (`self.Capture Scene on Begin Play`)
    (bind _outactors (`GameplayStatics.GetAllActorsOfClass` "/Game/StylizedRenderingSystem/Blueprints/BP_StylizedRenderingSystem.BP_StylizedRenderingSystem_C"))
    (for _array_element _outactors
      (bind _asstylized_rendering_system (cast `/Game/StylizedRenderingSystem/Blueprints/BP_StylizedRenderingSystem` _array_element :!pure true))
      (set `/Game/StylizedRenderingSystem/Blueprints/BP_StylizedRenderingSystem.Screen Percentage` (`self.Outline Scale (Screen Percentage Override)`) _asstylized_rendering_system)
      (`/Game/StylizedRenderingSystem/Blueprints/BP_StylizedRenderingSystem.Refresh` _asstylized_rendering_system))
    (`KismetSystemLibrary.PrintString` (`KismetStringLibrary.Concat_StrStr` "Stylized Rendering System: " "Reflection Component \"" _returnvalue "\" is beginning to capture your scene.") true true (struct :`R` 1.0 :`G` 0.25 :`A` 1.0) 10.0 (`KismetStringLibrary.Conv_StringToName` _returnvalue))
    (bind _returnvalue_3 (`AddComponent|NODE_AddSceneCaptureComponentCube-1`))
    (set `SceneCaptureComponentCube.TextureTarget` (`self.Texture Target`) _returnvalue_3)
    (`TimelineComponent.SetTimelineLength` (`self.Capture Timeline`) (`self.Capture Delay`))
    (`Timeline|Capture Timeline` :!via `PlayFromStart`
      (:`Update`
        (set `self.Cubemap` (`self.Texture Target`))
        (`self.Refresh`))
      (:`Finished`
        (`ActorComponent.K2_DestroyComponent` _returnvalue_3)
        (`KismetSystemLibrary.PrintString` (`KismetStringLibrary.Concat_StrStr` "Stylized Rendering System: " "Reflection Component \"" _returnvalue_2 "\" has successfully captured your scene. Make sure to disable capturing on this reflection component for performance.") true true (struct :`R` 0.25 :`G` 1.0 :`A` 1.0) 10.0 (`KismetStringLibrary.Conv_StringToName` _returnvalue_2))))))

(fn `Refresh`
  (bind _postprocess (`self.PostProcess`))
  (bind _mat_reflections (`self.Mat_Reflections`))
  (bind _secondary_bounds_size (`self.Secondary Bounds Size`))
  (bind _secondary_bounds (`self.Secondary Bounds`))
  (bind _secondary_bounds_outer_feather (`self.Secondary Bounds Outer Feather`))
  (bind _secondary_bounds_feathering (`self.Secondary Bounds Feathering`))
  (bind _primary_bounds_feather (`self.Primary Bounds Feather`))
  (bind _primary_bounds (`self.Primary Bounds`))
  (bind _returnvalue (`|EnumEquality` (`self.Blur Input Source`) "NewEnumerator1"))
  (bind _returnvalue_2 (`|EnumEquality` (`self.RS Input Source`) "NewEnumerator1"))
  (if (`self.Enable Reflection Volume`)
    ;[1 1 1] Limited to Bounds
    (if (`self.Use Primary Bounds`)
      (`SceneComponent.SetVisibility` _primary_bounds true false)
      (set `PostProcessComponent.bUnbound` (not (`self.Use Primary Bounds`)) _postprocess)
      (`BoxComponent.SetBoxExtent` _primary_bounds (`self.Primary Bounds Size`) true)
      (else
        (`SceneComponent.SetVisibility` _primary_bounds false false)
        (set `PostProcessComponent.bUnbound` true _postprocess)))
    ;[1 1 1] Primary Bounds Feather
    (if (and (!= (`self.Primary Bounds Feathering`) 0.0) (`self.Use Primary Bounds`))
      (`SceneComponent.SetVisibility` _primary_bounds_feather true false)
      (`BoxComponent.SetBoxExtent` _primary_bounds_feather (`KismetMathLibrary.Vector_ComponentMax` (- (`self.Primary Bounds Size`) (`self.Primary Bounds Feathering`))) true)
      (else
        (`SceneComponent.SetVisibility` _primary_bounds_feather false false)))
    ;[1 1 1] Secondary Bounds
    (if (`self.Use Secondary Bounds`)
      (`SceneComponent.SetVisibility` _secondary_bounds true false)
      (`BoxComponent.SetBoxExtent` _secondary_bounds (`self.Secondary Bounds Size`) true)
      (else
        (`SceneComponent.SetVisibility` _secondary_bounds false false)))
    ;[1 1 1] Secondary Bounds Feathering
    (if (and (!= (`self.Secondary Bounds Feathering`) 0.0) (`self.Use Secondary Bounds`))
      (`SceneComponent.SetVisibility` _secondary_bounds_outer_feather true false)
      (`SceneComponent.SetVisibility` (`self.Secondary Bounds Inner Feather`) true false)
      (`BoxComponent.SetBoxExtent` (`self.Secondary Bounds Inner Feather`) (`KismetMathLibrary.Vector_ComponentMax` (- _secondary_bounds_size _secondary_bounds_feathering)) true)
      (`BoxComponent.SetBoxExtent` (`self.Secondary Bounds Outer Feather`) (+ _secondary_bounds_size _secondary_bounds_feathering) true)
      (else
        (`SceneComponent.SetVisibility` _secondary_bounds_outer_feather false false)
        (`SceneComponent.SetVisibility` (`self.Secondary Bounds Inner Feather`) false false)))
    ;[1 1 1] Create Dynamic Material Instance for Reflection Volume
    (bind _returnvalue_3 (`KismetMaterialLibrary.CreateDynamicMaterialInstance` (`self.Reflection Material`) "Main"))
    (bind _output_get (set `self.Mat_Reflections` _returnvalue_3))
    (`KismetArrayLibrary.Array_Set` (`.Array` (break `WeightedBlendables` (`.WeightedBlendables` (break `PostProcessSettings` (`PostProcessComponent.Settings` (`self.PostProcess`)))))) 0 (make `WeightedBlendable` (select `/Game/StylizedRenderingSystem/Blueprints/Misc/BP_SRS_Modes_Enum` "NewEnumerator1" :`NewEnumerator1` 1.0 :`NewEnumerator0` 1.0) _output_get) true)
    (`|ExecutionSequence`
      (:`then_0`
        (`MaterialInstanceDynamic.SetTextureParameterValue` (`self.Mat_Reflections`) "Cubemap" (`self.Cubemap`))
        (`MaterialInstanceDynamic.SetScalarParameterValue` (`self.Mat_Reflections`) "Base Reflectivity" (`self.Base Reflectivity`))
        (`MaterialInstanceDynamic.SetScalarParameterValue` (`self.Mat_Reflections`) "Reflectivity Exponent" (`self.Reflectivity Exponent`)))
      (:`then_1`
        ;[1 1 1] Custom Depth and Stencil Mask
        (`MaterialInstanceDynamic.SetScalarParameterValue` (`self.Mat_Reflections`) "Only on Custom Depth" (`KismetMathLibrary.Conv_BoolToDouble` (`self.Only on Custom Depth`)))
        (`MaterialInstanceDynamic.SetScalarParameterValue` _mat_reflections "Stencil Mask Min" (`KismetMathLibrary.Conv_IntToDouble` (`self.Stencil Mask Min`)))
        (`MaterialInstanceDynamic.SetScalarParameterValue` _mat_reflections "Stencil Mask Max" (`KismetMathLibrary.Conv_IntToDouble` (`self.Stencil Mask Max`))))
      (:`then_2`
        ;[1 1 1] Bounds
        (`/Game/StylizedRenderingSystem/Blueprints/Misc/BP_StylizedRenderingSystem_FunctionLibrary.SetBoundsParameters` (`self.Mat_Reflections`) self (`self.Use Primary Bounds`) (`self.Primary Bounds Size`) (`self.Primary Bounds Feathering`) (`self.Bounds Behaviour`) (`self.Use Secondary Bounds`) (`self.Secondary Bounds Size`) (`self.Secondary Bounds Feathering`)))
      (:`then_3`
        ;[1 1 1] Reflection Strength Parameters
        (`MaterialInstanceDynamic.SetScalarParameterValue` (`self.Mat_Reflections`) "RS Metallic" (`self.RS Strength Metallic`))
        (`MaterialInstanceDynamic.SetScalarParameterValue` (`self.Mat_Reflections`) "RS non-Metallic" (`self.RS Strength non-Metallic`))
        (`MaterialInstanceDynamic.SetScalarParameterValue` (`self.Mat_Reflections`) "RS Input Source" (select `/Game/StylizedRenderingSystem/Blueprints/Misc/BP_SRS_ReflectionInputAssignment` (`self.RS Input Source`) :`NewEnumerator0` 1.0 :`NewEnumerator2` -1.0 :!type "Float (single-precision)"))
        (`MaterialInstanceDynamic.SetScalarParameterValue` (`self.Mat_Reflections`) "RS Min Highlight Size" (select `bool` _returnvalue_2 :`false` (`self.RS Min Highlight Size`) :`true` -1.0))
        (`MaterialInstanceDynamic.SetScalarParameterValue` (`self.Mat_Reflections`) "RS Max Highlight Size" (select `bool` _returnvalue_2 :`false` (`self.RS Max Highlight Size`) :`true` -0.99))
        (`MaterialInstanceDynamic.SetScalarParameterValue` (`self.Mat_Reflections`) "RS Min Rimlight Size" (select `bool` _returnvalue_2 :`false` (`self.RS Min Rimlight Size`) :`true` -1.0))
        (`MaterialInstanceDynamic.SetScalarParameterValue` (`self.Mat_Reflections`) "RS Max Rimlight Size" (select `bool` _returnvalue_2 :`false` (`self.RS Max Rimlight Size`) :`true` -0.99)))
      (:`then_4`
        ;[1 1 1] Blur Parameters
        (`MaterialInstanceDynamic.SetScalarParameterValue` (`self.Mat_Reflections`) "RB Metallic" (`self.RB Strength Metallic`))
        (`MaterialInstanceDynamic.SetScalarParameterValue` (`self.Mat_Reflections`) "RB non-Metallic" (`self.RB Strength non-Metallic`))
        (`MaterialInstanceDynamic.SetScalarParameterValue` (`self.Mat_Reflections`) "RB Input Source" (select `/Game/StylizedRenderingSystem/Blueprints/Misc/BP_SRS_ReflectionInputAssignment` (`self.Blur Input Source`) :`NewEnumerator0` 1.0 :`NewEnumerator2` -1.0 :!type "Float (single-precision)"))
        (`MaterialInstanceDynamic.SetScalarParameterValue` (`self.Mat_Reflections`) "RB Min Highlight Size" (select `bool` _returnvalue :`false` (`self.RB Min Highlight Size`) :`true` -1.0))
        (`MaterialInstanceDynamic.SetScalarParameterValue` (`self.Mat_Reflections`) "RB Max Highlight Size" (select `bool` _returnvalue :`false` (`self.RB Max Highlight Size`) :`true` -0.99))
        (`MaterialInstanceDynamic.SetScalarParameterValue` (`self.Mat_Reflections`) "RB Min Rimlight Size" (select `bool` _returnvalue :`false` (`self.RB Min Rimlight Size`) :`true` -1.0))
        (`MaterialInstanceDynamic.SetScalarParameterValue` (`self.Mat_Reflections`) "RB Max Rimlight Size" (select `bool` _returnvalue :`false` (`self.RB Max Rimlight Size`) :`true` -0.99))))))

(fn `UserConstructionScript`
  (`self.Refresh`))